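; AI controller for the Predator enemy that runs BT_Predator on possess and feeds it what it perceives of the player.
; Perception updates filter for BP_FirstPersonCharacter, setting the TargetActor blackboard key when the player is sensed.
; When the stimulus is lost, it stores the stimulus position as LastKnownLocation and clears TargetActor.
; Debug prints trace perception events and target acquisition.
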(event OnTargetPerceptionUpdated(AIPerception)
  (params (Actor :type Actor%20Object%20Reference) (Stimulus :type AI%20Stimulus%20Structure))
  (bind (_age _expirationage _strength _stimuluslocation _receiverlocation _tag _bsuccessfullysensed) (Utilities|Struct|BreakAIStimulus Stimulus))
  (bind _returnvalue (AI|GetBlackboard 0))
  (Development|PrintString "PERCEPTION FIRED")
  (bind _asbp_first_person_character (Utilities|Casting|CastToBP_FirstPersonCharacter Actor))
  (Development|PrintString "Player Cast Succeeded")
  (if _bsuccessfullysensed
    (Development|PrintString "SAW PLAYER - TRUE")
    (AI|Components|Blackboard|SetValueasObject _returnvalue (Utilities|Name|MakeLiteralName "TargetActor") _asbp_first_person_character)
    (Development|PrintString "TARGET ACTOR SET")
    (else
      (AI|Components|Blackboard|SetValueasVector _returnvalue (Utilities|Name|MakeLiteralName "LastKnownLocation") _stimuluslocation)
      (AI|Components|Blackboard|ClearValue _returnvalue (Utilities|Name|MakeLiteralName "TargetActor")))))

(event EventBeginPlay)

(event EventTick
  (params (DeltaSeconds :type Float%20%28single-precision%29)))

(event EventPossess
  (params (PossessedPawn :type Pawn%20Object%20Reference))
  (AI|RunBehaviorTree "/Game/Aphotia/AI/Predator/BehaviourTree/BT_Predator.BT_Predator"))

(fn ConstructionScript)