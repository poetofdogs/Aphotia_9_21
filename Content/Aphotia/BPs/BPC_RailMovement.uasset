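; BPC_RailMovement is a component that moves its owning Character along a rail axis.
; On BeginPlay it records the owner's starting X and Y and switches its Character Movement component to Flying mode.
; MoveAlongRail passes a scalar input to AddMovementInput along RailAxis while MovementEnabled is true.
; The stored start coordinates are not read in these graphs, so no position constraint is applied here.
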(event EventBeginPlay
  (bind _returnvalue (Components|GetOwner))
  (bind _returnvalue_2 (Transformation|GetActorLocation _returnvalue))
  (bind (_x _y) (Math|Vector|BreakVector _returnvalue_2))
  (Variables|Default|SetRailstartX _x)
  (Variables|Default|SetRailstartY _y)
  (bind _ascharacter (Utilities|Casting|CastToCharacter _returnvalue))
  (Pawn|Components|CharacterMovement|SetMovementMode (Actor|GetComponentbyClass _ascharacter "/Script/Engine.CharacterMovementComponent") "MOVE_Flying" 0))

(event EventTick
  (params (DeltaSeconds :type Float%20%28single-precision%29)))

(fn MoveAlongRail
  (params (MovementInput :type Float%20%28double-precision%29))
  (if (Variables|Default|GetbMovementEnabled)
    (bind _ascharacter (Utilities|Casting|CastToCharacter (Components|GetOwner)))
    (Pawn|Input|AddMovementInput _ascharacter (Variables|Default|GetRailAxis) MovementInput false)))